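; Player controller for a skill test, handling Enhanced Input for the controlled pawn, with BP_Myra-specific actions.
; It adds IMC_SkillTest on BeginPlay, then drives yaw-relative movement, look with optional pitch inversion, crouch toggling with debug prints, and jumping that uncrouches first.
; Sprint swaps max walk speed between BP_Myra's sprint and run values.
; The fire action casts a projectile on press, fires on completion and cancels if interrupted.
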(event `self.ReceiveBeginPlay`
  (`EnhancedInputSubsystemInterface.AddMappingContext` (subsystem `EnhancedInputLocalPlayerSubsystem`) "/Game/Characters/Allies/Myra/Inputs/IMC_SkillTest.IMC_SkillTest" 0 (struct)))

(event `EnhancedInput|/Game/Characters/Allies/Myra/Inputs/IA_Run`
  (params (ActionValue :type "Vector2D Structure") (ElapsedSeconds :type "Float (double-precision)") (TriggeredSeconds :type "Float (double-precision)") (InputAction :type "InputAction Object Reference" :default "/Game/Characters/Allies/Myra/Inputs/IA_Run.IA_Run"))
  (bind (_x _y) (`KismetMathLibrary.BreakVector2D` ActionValue))
  (bind (_returnvalue_roll _returnvalue_pitch _returnvalue_yaw) (`KismetMathLibrary.BreakRotator` (`self.GetControlRotation`)))
  (bind (_returnvalue_roll_2 _returnvalue_pitch_2 _returnvalue_yaw_2) (`KismetMathLibrary.BreakRotator` (`self.GetControlRotation`)))
  (:`Triggered`
    (`Pawn.AddMovementInput` (`self.K2_GetPawn`) (`KismetMathLibrary.GetForwardVector` (`KismetMathLibrary.MakeRotator` _returnvalue_roll_2 0.0 _returnvalue_yaw_2)) _y false) ; Forward
    (`Pawn.AddMovementInput` (`self.K2_GetPawn`) (`KismetMathLibrary.GetRightVector` (`KismetMathLibrary.MakeRotator` _returnvalue_roll 0.0 _returnvalue_yaw)) _x false) ; Right
  ))

(event `EnhancedInput|/Game/Characters/Allies/Myra/Inputs/IA_Sprint`
  (params (ActionValue :type Boolean) (ElapsedSeconds :type "Float (double-precision)") (TriggeredSeconds :type "Float (double-precision)") (InputAction :type "InputAction Object Reference" :default "/Game/Characters/Allies/Myra/Inputs/IA_Sprint.IA_Sprint"))
  (bind _asbp_myra (cast `/Game/Characters/Allies/Myra/BP_Myra` (`self.K2_GetPawn`) :!pure true))
  (bind _charactermovement (`Character.CharacterMovement` _asbp_myra))
  (:`Triggered`
    (set `CharacterMovementComponent.MaxWalkSpeed` (`/Game/Characters/Allies/Myra/BP_Myra.SprintSpeed` _asbp_myra) _charactermovement))
  (:`Completed`
    (set `CharacterMovementComponent.MaxWalkSpeed` (`/Game/Characters/Allies/Myra/BP_Myra.RunSpeed` _asbp_myra) _charactermovement)))

(event `EnhancedInput|/Game/Characters/Allies/Myra/Inputs/IA_Crouch`
  (params (ActionValue :type Boolean) (ElapsedSeconds :type "Float (double-precision)") (TriggeredSeconds :type "Float (double-precision)") (InputAction :type "InputAction Object Reference" :default "/Game/Characters/Allies/Myra/Inputs/IA_Crouch.IA_Crouch"))
  (bind _ascharacter (cast `Character` (`self.K2_GetPawn`) :!pure true))
  (:`Triggered`
    (if (`Character.bIsCrouched` _ascharacter)
      (`Character.UnCrouch` _ascharacter)
      (`KismetSystemLibrary.PrintString` "Uncrouch")
      (else
        (`Character.Crouch` _ascharacter)
        (`KismetSystemLibrary.PrintString` "Crouch")))))

(event `EnhancedInput|/Game/Characters/Allies/Myra/Inputs/IA_Look`
  (params (ActionValue :type "Vector2D Structure") (ElapsedSeconds :type "Float (double-precision)") (TriggeredSeconds :type "Float (double-precision)") (InputAction :type "InputAction Object Reference" :default "/Game/Characters/Allies/Myra/Inputs/IA_Look.IA_Look"))
  (bind (_x _y) (`KismetMathLibrary.BreakVector2D` ActionValue))
  (:`Triggered`
    (`self.AddYawInput` _x)
    (`self.AddPitchInput` (* _y (`KismetMathLibrary.SelectFloat` 1.0 -1.0 (`self.InvertAxis?`))))))

(event `EnhancedInput|/Game/Characters/Allies/Myra/Inputs/IA_FireProjectile`
  (params (ActionValue :type Boolean) (ElapsedSeconds :type "Float (double-precision)") (TriggeredSeconds :type "Float (double-precision)") (InputAction :type "InputAction Object Reference" :default "/Game/Characters/Allies/Myra/Inputs/IA_FireProjectile.IA_FireProjectile"))
  (:`Started`
    (bind _asbp_myra (cast `/Game/Characters/Allies/Myra/BP_Myra` (`self.K2_GetPawn`)))
    (`/Game/Characters/Allies/Myra/BP_Myra.CastProjectile` _asbp_myra))
  (:`Canceled`
    (bind _asbp_myra_2 (cast `/Game/Characters/Allies/Myra/BP_Myra` (`self.K2_GetPawn`)))
    (`/Game/Characters/Allies/Myra/BP_Myra.CancelProjectile` _asbp_myra_2))
  (:`Completed`
    (bind _asbp_myra_3 (cast `/Game/Characters/Allies/Myra/BP_Myra` (`self.K2_GetPawn`)))
    (`/Game/Characters/Allies/Myra/BP_Myra.FireProjectile` _asbp_myra_3)))

(event `EnhancedInput|/Game/Characters/Allies/Myra/Inputs/IA_Jump`
  (params (ActionValue :type Boolean) (ElapsedSeconds :type "Float (double-precision)") (TriggeredSeconds :type "Float (double-precision)") (InputAction :type "InputAction Object Reference" :default "/Game/Characters/Allies/Myra/Inputs/IA_Jump.IA_Jump"))
  (:`Started`
    (bind _ascharacter (cast `Character` (`self.K2_GetPawn`)))
    (`Character.UnCrouch` _ascharacter)
    (`Character.Jump` _ascharacter))
  (:`Completed`
    (bind _ascharacter_2 (cast `Character` (`self.K2_GetPawn`)))
    (`Character.StopJumping` _ascharacter_2)))

(fn `UserConstructionScript`)